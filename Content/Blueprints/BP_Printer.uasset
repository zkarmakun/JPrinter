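; BP_Printer exercises printer functions through four standalone events, with no triggers for them in its own graph.
; Two query events print the primary printer's name and each entry of the printer list as debug strings.
; Two print events send an image file path or a Texture2D to the primary printer, the texture on Letter paper.
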(event `Primary Printer`
  (`KismetSystemLibrary.PrintString` (`JPrinterBPLibrary.getPrimaryPrinterName`)))

(event `All Printers`
  (for _array_element (`JPrinterBPLibrary.getPrinterList`)
    (`KismetSystemLibrary.PrintString` _array_element)))

(event `Print Image`
  (`JPrinterBPLibrary.printImage` (`self.ImageToPrintPath`)))

(event `Print Texture`
  (`JPrinterBPLibrary.printTexture2D` (`self.TextureToPrint`) "" true "letter"))

(fn `UserConstructionScript`)